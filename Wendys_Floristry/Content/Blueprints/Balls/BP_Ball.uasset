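; BP_Ball is a ball actor that can be harvested through interaction and can replace itself with a color-specific variant.
; OnInteract, while the ball is visible, hides its mesh, disables collision and prints a harvest message, so it only fires once while visible.
; CreateChildActor maps a ball color enum to one of seven colored BP_Ball subclasses, spawns it at the same transform, then destroys the original.
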(event EventOnInteract
  (if (Variables|Default|GetisVisible)
    (bind _output_get (Variables|Default|SetisVisible (not (Variables|Default|GetisVisible))))
    (Rendering|SetVisibility (Variables|Default|GetBall) _output_get false)
    (Collision|SetActorEnableCollision _output_get)
    (Development|PrintText (Utilities|Text|FormatText "Harvest: {Name}" (Utilities|GetObjectName self)))))

(fn ConstructionScript)

(fn CreateChildActor
  (params (EnumBallColor :type Enum_Ball_Colors%20Enum :default "NewEnumerator0"))
  (bind _returnvalue (Transformation|GetActorTransform))
  (switch Utilities|FlowControl|Switch|SwitchonEnum_Ball_Colors EnumBallColor
    (:NewEnumerator0
      (Game|SpawnActorfromClass "/Game/Blueprints/Balls/BP_Ball_Red.BP_Ball_Red_C" _returnvalue "Undefined" "MultiplyWithRoot" 0 0))
    (:NewEnumerator1
      (Game|SpawnActorfromClass "/Game/Blueprints/Balls/BP_Ball_Blue.BP_Ball_Blue_C" _returnvalue "Undefined" "MultiplyWithRoot" 0 0))
    (:NewEnumerator2
      (Game|SpawnActorfromClass "/Game/Blueprints/Balls/BP_Ball_White.BP_Ball_White_C" _returnvalue "Undefined" "MultiplyWithRoot" 0 0))
    (:NewEnumerator3
      (Game|SpawnActorfromClass "/Game/Blueprints/Balls/BP_Ball_Orange.BP_Ball_Orange_C" _returnvalue "Undefined" "MultiplyWithRoot" 0 0))
    (:NewEnumerator4
      (Game|SpawnActorfromClass "/Game/Blueprints/Balls/BP_Ball_Yellow.BP_Ball_Yellow_C" _returnvalue "Undefined" "MultiplyWithRoot" 0 0))
    (:NewEnumerator5
      (Game|SpawnActorfromClass "/Game/Blueprints/Balls/BP_Ball_Pink.BP_Ball_Pink_C" _returnvalue "Undefined" "MultiplyWithRoot" 0 0))
    (:NewEnumerator6
      (Game|SpawnActorfromClass "/Game/Blueprints/Balls/BP_Ball_Purple.BP_Ball_Purple_C" _returnvalue "Undefined" "MultiplyWithRoot" 0 0)))
  (Actor|DestroyActor))