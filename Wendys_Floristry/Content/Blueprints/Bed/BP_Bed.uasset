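; Interactable bed that lets the player sleep to start a new day.
; Holding F through the interaction delay has BP_Player display the sleep confirmation widget.
; Sleep, not called within this Blueprint, re-triggers the map's PCG controller and resets the day-night cycle's light rotation and lights to day.
; A separate helper reports whether the customer table still has customers.
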(event EventOnInteract
  (Utilities|FlowControl|Delay (Variables|Default|GetinteractTime))
  (if (Game|Player|IsInputKeyDown (Game|GetPlayerController 0) "F")
    (bind _returnvalue (Actor|GetActorOfClass "/Game/Blueprints/Player/BP_Player.BP_Player_C"))
    (Default|DisplayUI _returnvalue "/Game/Blueprints/Widgets/WBP_SleepConfirm.WBP_SleepConfirm_C")))

(fn ConstructionScript)

(fn CheckLeftoverCustomer
  (bind _returnvalue (Actor|GetActorOfClass "/Game/Blueprints/Customer/BP_CustomerTable.BP_CustomerTable_C"))
  (return (> (Utilities|Map|Length (Variables|/Game/Blueprints/Customer/BP_CustomerTable.BP_CustomerTable_C|GetcustomerList _returnvalue)) 0)))

(fn Sleep
  (bind _returnvalue (Actor|GetActorOfClass "/Game/Levels/PCG/BP_Map_PCGController.BP_Map_PCGController_C"))
  (Default|TriggerPCGV _returnvalue)
  (bind _returnvalue_2 (Actor|GetActorOfClass "/Game/Blueprints/DayNightCycle/BP_DayNightCycle.BP_DayNightCycle_C"))
  (Variables|/Game/Blueprints/DayNightCycle/BP_DayNightCycle.BP_DayNightCycle_C|SetLightRotation _returnvalue_2 "10.000000,150.000000,0.000000")
  (bind _output_get (Variables|/Game/Blueprints/DayNightCycle/BP_DayNightCycle.BP_DayNightCycle_C|SetisNight _returnvalue_2 false))
  (Default|SwitchLights _returnvalue_2 _output_get)
  (return))