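; Customer table that generates flower orders at BeginPlay and opens the customer data screen on the player.
; Reads DayCount from BP_DayNightCycle to scale customer count, flowers per order and score per flower in three difficulty tiers.
; Randomly spreads each order across seven colors, storing it in the CustomerList map by index.
; OnInteract waits InteractTime and shows WBP_CustomerDataScreen only if F is still down.
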(event EventBeginPlay
  (CallFunction|GetDayCount)
  (CallFunction|RandomCustomerCount)
  (CallFunction|RandomCustomerData))

(event EventOnInteract
  (Utilities|FlowControl|Delay (Variables|Default|GetInteractTime))
  (if (Game|Player|IsInputKeyDown (Game|GetPlayerController 0) "F")
    (bind _returnvalue (Actor|GetActorOfClass "/Game/Blueprints/Player/BP_Player.BP_Player_C"))
    (Default|DisplayUI _returnvalue "/Game/Blueprints/Widgets/WBP_CustomerDataScreen.WBP_CustomerDataScreen_C")))

(fn ConstructionScript)

(fn RandomCustomerCount
  (bind _daycount (Variables|Default|GetdayCount))
  (bind _returnvalue (+ _daycount 2))
  (Variables|Default|SetcustomerCount (Math|Random|RandomIntegerinRange (Math|Integer|Clamp(Integer) (- _daycount 2) 2 _returnvalue) _returnvalue))
  (return))

(fn RandomCustomerData
  (bind _flowercountlist (LocalVariables|GetflowerCountList))
  (Utilities|Map|Clear (Variables|Default|GetcustomerList))
  (for _index (range 0 (- (Variables|Default|GetcustomerCount) 1))
    (if (<= (Variables|Default|GetdayCount) 4)
      (LocalVariables|SetflowerCount (Math|Conversions|ToByte(Integer) (Math|Random|RandomIntegerinRange 1 4)))
      (LocalVariables|SetscorePerFlower 10)
      (elif (<= (Variables|Default|GetdayCount) 7)
        (LocalVariables|SetflowerCount (Math|Conversions|ToByte(Integer) (Math|Random|RandomIntegerinRange 3 7)))
        (LocalVariables|SetscorePerFlower 15)
        (else
          (LocalVariables|SetflowerCount (Math|Conversions|ToByte(Integer) (Math|Random|RandomIntegerinRange 4 9)))
          (LocalVariables|SetscorePerFlower 25))))
    (for (_ _array_index) _flowercountlist
      (Utilities|Array|SetArrayElem _flowercountlist _array_index 0))
    (for _index_2 (range 0 (- (LocalVariables|GetflowerCount) 1))
      (bind _output_get (LocalVariables|SetrandomFlowerIndex (Math|Random|RandomIntegerinRange 0 6)))
      (Utilities|Array|SetArrayElem (LocalVariables|GetflowerCountList) _output_get (+ (Utilities|Array|Get(acopy) (LocalVariables|GetflowerCountList) _output_get) 1)))
    (Utilities|Map|Add (Variables|Default|GetcustomerList) _index (Utilities|Struct|MakeST_CustomerData 0 (Utilities|Array|Get(acopy) (LocalVariables|GetflowerCountList)) (Utilities|Array|Get(acopy) (LocalVariables|GetflowerCountList) 1) (Utilities|Array|Get(acopy) (LocalVariables|GetflowerCountList) 2) (Utilities|Array|Get(acopy) (LocalVariables|GetflowerCountList) 3) (Utilities|Array|Get(acopy) (LocalVariables|GetflowerCountList) 4) (Utilities|Array|Get(acopy) (LocalVariables|GetflowerCountList) 5) (Utilities|Array|Get(acopy) (LocalVariables|GetflowerCountList) 6) (* (LocalVariables|GetflowerCount) (LocalVariables|GetscorePerFlower)))))
  (return))

(fn GetDayCount
  (bind _returnvalue (Actor|GetActorOfClass "/Game/Blueprints/DayNightCycle/BP_DayNightCycle.BP_DayNightCycle_C"))
  (Variables|Default|SetdayCount (Variables|/Game/Blueprints/DayNightCycle/BP_DayNightCycle.BP_DayNightCycle_C|GetdayCount _returnvalue))
  (return))

(fn DisplayCustomerData
  (for _index (range 0 (- (Utilities|Map|Length (Variables|Default|GetcustomerList)) 1))
    (Development|PrintText (Utilities|Text|FormatText "Index: {Index} 
Red: {Red} 
Blue: {Blue} 
White: {White} 
Orange: {Orange} 
Yellow: {Yellow} 
Pink: {Pink} 
Purple: {Purple} 
Score: {Score}" _index (.RedFlowerCount (Utilities|Struct|BreakST_CustomerData (.Value (Utilities|Map|Find (Variables|Default|GetcustomerList) _index)))) (.BlueFlowerCount (Utilities|Struct|BreakST_CustomerData (.Value (Utilities|Map|Find (Variables|Default|GetcustomerList) _index)))) (.WhiteFlowerCount (Utilities|Struct|BreakST_CustomerData (.Value (Utilities|Map|Find (Variables|Default|GetcustomerList) _index)))) (.OrangeFlowerCount (Utilities|Struct|BreakST_CustomerData (.Value (Utilities|Map|Find (Variables|Default|GetcustomerList) _index)))) (.YellowFlowerCount (Utilities|Struct|BreakST_CustomerData (.Value (Utilities|Map|Find (Variables|Default|GetcustomerList) _index)))) (.PinkFlowerCount (Utilities|Struct|BreakST_CustomerData (.Value (Utilities|Map|Find (Variables|Default|GetcustomerList) _index)))) (.PurpleFlowerCount (Utilities|Struct|BreakST_CustomerData (.Value (Utilities|Map|Find (Variables|Default|GetcustomerList) _index)))) (.CustomerScore (Utilities|Struct|BreakST_CustomerData (.Value (Utilities|Map|Find (Variables|Default|GetcustomerList) _index)))))))
  (return))