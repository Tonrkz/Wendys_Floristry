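; Day/night cycle actor that pitches the day and night lights each tick while GameStart is set, toggling their visibility at a sunset threshold.
; Day and night durations are converted to degrees-per-second rates, and each phase change updates IsNight on every BP_BaseCat.
; Each new day after the first adds a random score from a rising range, lengthens both phases, nights faster, and notifies every BP_Den.
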(event EventBeginPlay
  (Variables|Default|SetisNight false)
  (Variables|Default|SetLightRotation "10.000000,150.000000,0.000000")
  (bind _output_get (Variables|Default|SetSunSetDegreeTreshold -1.8e+02))
  (Variables|Default|SetDegreePerHalfDay (Math|Float|Absolute(Float) (+ _output_get (.pitch (stale EventTick _output_get_3)))))
  (Variables|Default|SetdayCount -1)
  (Variables|Default|SetdayScore 0)
  (Variables|Default|SetdayScoreMinRange 1200)
  (Variables|Default|SetdayScoreMaxRange 1500)
  (CallFunction|CalculateTimeCount (Variables|Default|GetDayTimeSeconds) (Variables|Default|GetNightTimeSeconds))
  (CallFunction|SwitchLights (Variables|Default|GetisNight)))

(event EventTick
  (params (DeltaSeconds :type Float%20%28single-precision%29))
  (if (Variables|Default|GetgameStart)
    (if (Variables|Default|GetisNight)
      (bind _output_get (Variables|Default|SetLightRotation (Math|Rotator|MakeRotator (.roll (Variables|Default|GetLightRotation)) (- (.pitch (Variables|Default|GetLightRotation)) (* DeltaSeconds (Variables|Default|GetNightTimeSeconds))) (.yaw (Variables|Default|GetLightRotation)))))
      (CallFunction|RotateLights _output_get)
      (else
        (bind _output_get_2 (Variables|Default|SetLightRotation (Math|Rotator|MakeRotator (.roll (Variables|Default|GetLightRotation)) (- (.pitch (Variables|Default|GetLightRotation)) (* DeltaSeconds (Variables|Default|GetDayTimeSeconds))) (.yaw (Variables|Default|GetLightRotation)))))
        (CallFunction|RotateLights _output_get_2)))
    (if (<= (.Pitch (Math|Rotator|BreakRotator (Variables|Default|GetLightRotation))) (Variables|Default|GetSunSetDegreeTreshold))
      (bind _output_get_3 (Variables|Default|SetLightRotation "-10.000000,150.000000,0.000000"))
      (bind _output_get_4 (Variables|Default|SetisNight (not (Variables|Default|GetisNight))))
      (CallFunction|SetCatDayNight _output_get_4)
      (CallFunction|SwitchLights _output_get_4))))

(fn ConstructionScript)

(fn SwitchLights
  (params (isNight :type Boolean))
  (bind _daylight (Variables|Default|GetDayLight))
  (bind _nightlight (Variables|Default|GetNightLight))
  (if isNight
    (Rendering|SetVisibility (Variables|/Script/Engine.Light|GetLightComponent _daylight) false true)
    (Rendering|SetVisibility (Variables|/Script/Engine.Light|GetLightComponent _nightlight) true true)
    (else
      (Rendering|SetVisibility (Variables|/Script/Engine.Light|GetLightComponent _daylight) true true)
      (Rendering|SetVisibility (Variables|/Script/Engine.Light|GetLightComponent _nightlight) false true)
      (CallFunction|NewDay)))
  (return))

(fn RotateLights
  (params (Rotation :type Rotator))
  (Transformation|SetActorRotation (Variables|Default|GetDayLight) Rotation true)
  (Transformation|SetActorRotation (Variables|Default|GetNightLight) Rotation true)
  (return))

(fn CalculateTimeCount
  (params (DayTimeCount :type Float%20%28double-precision%29) (NightTimeCount :type Float%20%28double-precision%29))
  (bind _degreeperhalfday (Variables|Default|GetDegreePerHalfDay))
  (Variables|Default|SetDayTimeSeconds (/ _degreeperhalfday DayTimeCount))
  (Variables|Default|SetNightTimeSeconds (/ _degreeperhalfday NightTimeCount))
  (return))

(fn NewDay
  (bind _daycount (Variables|Default|GetdayCount))
  (Math|Integer|IncrementInt _daycount
    (:%20%20
      (if (>= _daycount 1)
        (bind _output_get (Variables|Default|SetdayScoreMinRange (+ (Variables|Default|GetdayScoreMinRange) 50)))
        (bind _output_get_2 (Variables|Default|SetdayScoreMaxRange (+ (Variables|Default|GetdayScoreMaxRange) 50)))
        (bind _output_get_3 (Variables|Default|SetdayScore (+ (Variables|Default|GetdayScore) (Math|Random|RandomIntegerinRange _output_get _output_get_2))))
        (Development|PrintText (Utilities|Text|FormatText "Day Score: {daySocre}" _output_get_3))
        (bind (_newdaytimesecond _newnighttimeseconds) (CallFunction|ExtendDayNightTime (Variables|Default|GetDayTimeSeconds) 1.03 (Variables|Default|GetNightTimeSeconds) 1.05))
        (CallFunction|CalculateTimeCount _newdaytimesecond _newnighttimeseconds)
        (bind _outactors (Actor|GetAllActorsOfClass "/Game/Blueprints/Den/BP_Den.BP_Den_C"))
        (for _array_element _outactors
          (Class|BPIDenNewDay|DenNewDay(Message) _array_element (+ (Variables|Default|GetdayCount) 1)))
        (return)))))

(fn ExtendDayNightTime
  (params (dayTimeSecond :type Float%20%28double-precision%29) (dayTimeMultiplier :type Float%20%28double-precision%29) (nightTimeSecond :type Float%20%28double-precision%29) (nightTimeMultiplier :type Float%20%28double-precision%29))
  (bind _degreeperhalfday (Variables|Default|GetDegreePerHalfDay))
  (return (* (/ _degreeperhalfday dayTimeSecond) dayTimeMultiplier) (* (/ _degreeperhalfday nightTimeSecond) nightTimeMultiplier)))

(fn SetCatDayNight
  (params (isNight :type Boolean))
  (bind _outactors (Actor|GetAllActorsOfClass "/Game/Blueprints/Enemies/BP_BaseCat.BP_BaseCat_C"))
  (for _array_element _outactors
    (Variables|/Game/Blueprints/Enemies/BP_BaseCat.BP_BaseCat_C|SetisNight _array_element isNight))
  (return))