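; BP_Den is a cat den that spawns a batch of AI cats on each new day event.
; Every third day it raises MaxCatCount by two, then spawns that full count without checking for existing cats.
; Each cat gets a random color variant and navigable spot near the den, runs the day behavior tree, and stores the den in its blackboard as DenActor.
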(event EventDenNewDay
  (params (dayCount :type Integer))
  (Utilities|FlowControl|Sequence
    (:then_0
      (if (== (Math|Integer|%(Integer) dayCount 3) 0)
        (CallFunction|UpdateMaxCatCount)))
    (:then_1
      (CallFunction|SpawnCat))))

(fn ConstructionScript)

(fn UpdateMaxCatCount
  (Variables|Default|SetmaxCatCount (+ (Variables|Default|GetmaxCatCount) 2))
  (return))

(fn SpawnCat
  (for _index (range 1 (Variables|Default|GetmaxCatCount))
    (bind _randomlocation (Class|NavigationSystemV1|GetRandomLocationinNavigableRadius (Transformation|GetActorLocation self) 6.4e+02 0 0))
    (bind _returnvalue (AI|SpawnAIFromClass (Utilities|Select :Index (Math|Random|RandomIntegerinRange 0 3) :Option%200 "/Game/Blueprints/Enemies/BP_BaseCat.BP_BaseCat_C" :Option%201 "/Game/Blueprints/Enemies/BP_BaseCat_Black.BP_BaseCat_Black_C" :Option%202 "/Game/Blueprints/Enemies/BP_BaseCat_BlackAndWhite.BP_BaseCat_BlackAndWhite_C" :Option%203 "/Game/Blueprints/Enemies/BP_BaseCat_White.BP_BaseCat_White_C") "/Game/Blueprints/Enemies/BehaviorTrees/BT_BaseCat_Day.BT_BaseCat_Day" _randomlocation "0, 0, 0" false 0))
    (AI|Components|Blackboard|SetValueasObject (AI|GetBlackboard (AI|GetAIController _returnvalue)) (Utilities|Name|MakeLiteralName "DenActor") self))
  (return))