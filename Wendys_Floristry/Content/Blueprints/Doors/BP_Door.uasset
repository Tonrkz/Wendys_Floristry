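; Double door Blueprint that toggles open and closed on an interact event.
; OnInteract waits for InteractTime, then proceeds only if F is down at that moment, approximating a hold-to-interact.
; IsOpen selects whether a Timeline plays forward or reverses from its end, driving the yaw of Door1 and Door2 through separate tracks.
; Each Timeline update also prints a debug message.
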(event EventOnInteract
  (Utilities|FlowControl|Delay (Variables|Default|GetInteractTime))
  (if (Game|Player|IsInputKeyDown (Game|GetPlayerController 0) "F")
    (if (Variables|Default|GetisOpen)
      (Variables|Default|SetisOpen (not (Variables|Default|GetisOpen)))
      (bind (_direction _door_2_z_rotation _door_1_z_rotation) (Timeline|Timeline ReverseFromEnd)
        (:Update
          (Transformation|SetRelativeRotation (Variables|Default|GetDoor_2) (Math|Rotator|MakeRotator 0.0 0.0 _door_2_z_rotation) false false)
          (Transformation|SetRelativeRotation (Variables|Default|GetDoor_1) (Math|Rotator|MakeRotator 0.0 0.0 _door_1_z_rotation) false false)
          (Development|PrintString "Interacted: Door")))
      (else
        (Variables|Default|SetisOpen (not (Variables|Default|GetisOpen)))
        (Timeline|Timeline Play)))))

(fn ConstructionScript)