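; AI controller for cat enemies that starts BT_BaseCat in WalkAround and switches to Attack on seeing the player.
; Sight perception of an exact BP_Player class writes AttackTargetActor to the Blackboard, refreshing it if already attacking.
; SetState mirrors BaseCatState to the Blackboard; nothing here returns it to WalkAround.
; SetMoveSpeed, not called here, maps walk, sprint and freeze to movement speed on the owner cast to BP_BaseCat.
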(event OnTargetPerceptionUpdated(AIPerception)
  (params (Actor :type Actor%20Object%20Reference) (Stimulus :type AI%20Stimulus%20Structure))
  (bind _returnvalue (Class|AIPerceptionSystem|GetSenseClassforStimulus Stimulus))
  (if (and (== _returnvalue "/Script/AIModule.AISense_Sight") (== (Utilities|GetClass Actor) "/Game/Blueprints/Player/BP_Player.BP_Player_C"))
    (bind _currentstate (CallFunction|GetCurrentState))
    (switch Utilities|FlowControl|Switch|SwitchonEnum_BaseCatState _currentstate
      (:NewEnumerator0
        _)
      (:NewEnumerator1
        _))
    (CallFunction|SetState "NewEnumerator1")
    (AI|Components|Blackboard|SetValueasObject (AI|GetBlackboard 0) (Utilities|Name|MakeLiteralName "AttackTargetActor") Actor)))

(event EventBeginPlay
  (AI|RunBehaviorTree "/Game/Blueprints/Enemies/BehaviorTrees/BT_BaseCat.BT_BaseCat")
  (CallFunction|SetState "NewEnumerator0"))

(fn ConstructionScript)

(fn SetState
  (params (State :type Enum_BaseCatState%20Enum :default "NewEnumerator0"))
  (bind _output_get (Variables|Default|SetBaseCatState State))
  (AI|Components|Blackboard|SetValueasEnum (AI|GetBlackboard 0) (Utilities|Name|MakeLiteralName "BaseCatState") _output_get)
  (return))

(fn GetCurrentState
  (return (Variables|Default|GetBaseCatState)))

(fn SetMoveSpeed
  (params (Speed :type Enum_BaseCat_MoveSpeed%20Enum :default "NewEnumerator0"))
  (bind _asbp_base_cat (Utilities|Casting|CastToBP_BaseCat (Components|GetOwner self)))
  (Variables|Default|SetMoveSpeed Speed)
  (switch Utilities|FlowControl|Switch|SwitchonEnum_BaseCat_MoveSpeed Speed
    (:NewEnumerator0
      (Variables|/Script/Engine.CharacterMovementComponent|SetMaxWalkSpeed (Variables|/Script/Engine.Character|GetCharacterMovement _asbp_base_cat) 2e+02))
    (:NewEnumerator1
      (Variables|/Script/Engine.CharacterMovementComponent|SetMaxWalkSpeed (Variables|/Script/Engine.Character|GetCharacterMovement _asbp_base_cat) 4e+02))
    (:NewEnumerator2
      (Variables|/Script/Engine.CharacterMovementComponent|SetMaxWalkSpeed (Variables|/Script/Engine.Character|GetCharacterMovement _asbp_base_cat) 0.0)))
  (return))