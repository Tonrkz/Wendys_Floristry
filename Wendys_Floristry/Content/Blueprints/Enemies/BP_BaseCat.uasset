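; Base enemy cat whose stats scale with the day count from BP_DayNightCycle and rise at night.
; SetBaseCatStat feeds the health and status components, while the IsNight RepNotify also updates the AI blackboard.
; Incoming damage is reduced by DEF and gated by a DoOnce until AttackEnd, playing hit or random death montages and awarding score on death.
; AttackHitHandler passes attack damage to BP_Player.
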(event EventBeginPlay
  (bind _acbp_health_system (Variables|Default|GetACBP_Health_System))
  (bind _returnvalue (Actor|GetActorOfClass "/Game/Blueprints/DayNightCycle/BP_DayNightCycle.BP_DayNightCycle_C"))
  (Variables|Default|SetdayCount (+ (Variables|/Game/Blueprints/DayNightCycle/BP_DayNightCycle.BP_DayNightCycle_C|GetdayCount _returnvalue) 1))
  (CallFunction|SetBaseCatStat 1.0)
  (Variables|/Game/Blueprints/Player/ACBP_Health_System.ACBP_Health_System_C|SetHP _acbp_health_system (Variables|/Game/Blueprints/Player/ACBP_Health_System.ACBP_Health_System_C|GetmaxHP _acbp_health_system)))

(event EventDamageResponseHandler
  (params (Damage :type Float%20%28double-precision%29))
  (bind _returnvalue (/ Damage 2.0))
  (bind _acbp_health_system (Variables|Default|GetACBP_Health_System))
  (bind _acbp_status_system (Variables|Default|GetACBP_Status_System))
  (bind _def (Variables|/Game/Blueprints/Player/ACBP_Status_System.ACBP_Status_System_C|GetDEF _acbp_status_system))
  (bind _returnvalue_2 (- Damage _def))
  (bind _returnvalue_3 (Math|Float|Clamp(Float) _returnvalue_2 _returnvalue Damage))
  ;[0.05098 0.05098 0.05098] Hit Response
  (Utilities|FlowControl|DoOnce false
    (:Completed
      (if (> Damage 0.0)
        (Development|PrintText (Utilities|Text|FormatText "Cat Took {DMG} Damage!" _returnvalue_3))
        (bind _output_get (Variables|/Game/Blueprints/Player/ACBP_Health_System.ACBP_Health_System_C|SetHP _acbp_health_system (Math|Float|Clamp(Float) (- (Variables|/Game/Blueprints/Player/ACBP_Health_System.ACBP_Health_System_C|GetHP _acbp_health_system) _returnvalue_3))))
        (if (<= _output_get 0.0)
          (Utilities|FlowControl|DoOnce false
            (:Completed
              (Pawn|Components|CharacterMovement|DisableMovement (Variables|Character|GetCharacterMovement))
              (if (Math|Random|RandomBool)
                (Animation|Montage|PlayMontage (Variables|Character|GetMesh) "/Game/DownloadedAssets/LowPoly_Cat/Animations/AM_Cat_Death_L.AM_Cat_Death_L"
                  (:OnCompleted
                    _)
                  (:OnInterrupted
                    _))
                (else
                  (Animation|Montage|PlayMontage (Variables|Character|GetMesh) "/Game/DownloadedAssets/LowPoly_Cat/Animations/AM_Cat_Death_R.AM_Cat_Death_R"
                    (:OnCompleted
                      _)
                    (:OnInterrupted
                      _))))
              (bind _returnvalue_4 (Actor|GetActorOfClass "/Game/Blueprints/Player/BP_Player.BP_Player_C"))
              (Variables|/Game/Blueprints/Player/ACBP_Score_System.ACBP_Score_System_C|SetScore (Variables|/Game/Blueprints/Player/BP_Player.BP_Player_C|GetACBP_Score_System _returnvalue_4) (+ (Variables|/Game/Blueprints/Player/ACBP_Score_System.ACBP_Score_System_C|GetScore (Variables|/Game/Blueprints/Player/BP_Player.BP_Player_C|GetACBP_Score_System _returnvalue_4)) (.score (Variables|Default|GetBaseCatStat))))
              (Actor|DestroyActor)))
          (else
            (Components|Movement|StopMovementImmediately (Variables|Character|GetCharacterMovement))
            (Animation|Montage|PlayMontage (Variables|Character|GetMesh) "/Game/DownloadedAssets/LowPoly_Cat/Animations/AM_Cat_Hit_F.AM_Cat_Hit_F")))))))

(event EventAttackEnd
  (params (HitActor :type Actor%20Object%20Reference))
  (bind _acbp_health_system (Variables|Default|GetACBP_Health_System))
  ;[0.05098 0.05098 0.05098] Hit Response
  (if (== (Utilities|GetClass HitActor) "BP_BaseCat_C")
    (Utilities|FlowControl|DoOnce false) ; enters at Reset
  ))

(event EventDenNewDay
  (params (dayCount :type Integer))
  (Variables|Default|SetdayCount dayCount)
  (CallFunction|SetBaseCatStat 1.0))

(fn ConstructionScript)

(fn SetBaseCatStat
  (params (Multiplier :type Float%20%28double-precision%29))
  (bind _returnvalue (Math|Float|MakeLiteralFloat 9.0))
  (bind _returnvalue_2 (Class|KismetSystemLibrary|MakeLiteralInteger 9))
  (bind _daycount (Variables|Default|GetdayCount))
  (bind _acbp_health_system (Variables|Default|GetACBP_Health_System))
  (bind _acbp_status_system (Variables|Default|GetACBP_Status_System))
  (bind _returnvalue_3 (Math|Conversions|ToFloat(Integer) _daycount))
  (bind _returnvalue_4 (/ _returnvalue_3 3.0))
  (bind _returnvalue_5 (* _returnvalue _returnvalue_4 Multiplier))
  (bind _returnvalue_6 (* _returnvalue_2 _returnvalue_4 Multiplier))
  (bind _output_get (Variables|Default|SetBaseCatStat (Utilities|Struct|MakeST_BaseCatStat 1e+01 _returnvalue_5 _returnvalue_5 _returnvalue_6 3 (Math|Random|RandomIntegerinRange (- _returnvalue_6 2) (+ _returnvalue_6 2)))))
  (bind _output_get_2 (Variables|/Game/Blueprints/Player/ACBP_Health_System.ACBP_Health_System_C|SetmaxHP _acbp_health_system (.maxhp _output_get)))
  (Variables|/Game/Blueprints/Player/ACBP_Health_System.ACBP_Health_System_C|SetRegenHP _acbp_health_system (.regenhp _output_get))
  (Variables|/Game/Blueprints/Player/ACBP_Status_System.ACBP_Status_System_C|SetATK _acbp_status_system (.atk _output_get))
  (Variables|/Game/Blueprints/Player/ACBP_Status_System.ACBP_Status_System_C|SetDEF _acbp_status_system (.def _output_get))
  (if (> (Variables|/Game/Blueprints/Player/ACBP_Health_System.ACBP_Health_System_C|GetHP _acbp_health_system) _output_get_2)
    (Variables|/Game/Blueprints/Player/ACBP_Health_System.ACBP_Health_System_C|SetHP _acbp_health_system _output_get_2)))

(fn OnRepIsNight
  (bind _isnight (Variables|Default|GetisNight))
  (AI|Components|Blackboard|SetValueasBool (AI|GetBlackboard (AI|GetAIController self)) (Utilities|Name|MakeLiteralName "isNight") _isnight)
  (if _isnight
    (CallFunction|SetBaseCatStat 1.5)
    (else
      (CallFunction|SetBaseCatStat 1.0))))

(fn AttackHitHandler
  (params (HitActor :type Actor%20Object%20Reference))
  (bind _asbp_player (Utilities|Casting|CastToBP_Player HitActor))
  (Class|BPIDamagable|DamageResponseHandler(Message) _asbp_player (.Damage (Utilities|Struct|BreakST_AttackInfo (Variables|Default|GetAttackData))))
  (return))