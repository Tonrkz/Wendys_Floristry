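; BP_Flower is a harvestable flower actor that adds its color to the player's inventory.
; OnHarvest waits for a delay scaled by harvest speed, then proceeds only if F is down and the flower is visible.
; A DoOnce then hides the flower, disables collision, updates the inventory and clears the player's interacting and harvesting flags.
; The construction script randomizes the flower's score.
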(event EventOnHarvest
  (params (harvestSpeed :type Float%20%28double-precision%29) (InventorySystem :type ACBP%20Inventory%20System%20Object%20Reference%20%28by%20ref%29))
  (Utilities|FlowControl|Delay (/ (Variables|Default|GetharvestTime) harvestSpeed))
  (if (and (Game|Player|IsInputKeyDown (Game|GetPlayerController 0) "F") (Variables|Default|GetisVisible))
    (Utilities|FlowControl|DoOnce false
      (:Completed
        (bind _output_get (Variables|Default|SetisVisible (not (Variables|Default|GetisVisible))))
        (Rendering|SetVisibility (Variables|Default|GetFlower) _output_get true)
        (Collision|SetActorEnableCollision _output_get)
        (Development|PrintText (Utilities|Text|FormatText "Harvest: {Name}" (Utilities|GetObjectName self)))
        (Default|AddFlowertoInventory InventorySystem (Variables|Default|GetFlowerColor))
        (bind _asbp_player (Utilities|Casting|CastToBP_Player (Game|Player|GetPlayerPawn 0)))
        (Variables|/Game/Blueprints/Player/BP_Player.BP_Player_C|SetisInteracting _asbp_player false)
        (Variables|/Game/Blueprints/Player/BP_Player.BP_Player_C|SetisHarvesting _asbp_player false)))))

(fn ConstructionScript
  (Variables|Default|SetFlowerScore (Math|Random|RandomIntegerinRange 10 20)))