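; Anim notify state that runs melee hit detection for cat enemies and the player during attack montages.
; Each tick it sphere-traces pawns, picking the cat's mouth, left-claw or right-claw socket by montage name, or sweeping between two right-hand sockets for the player.
; Cats only hit BP_Player, the player hits non-player BPI_Damagable actors, and the first valid hit per tick goes to the attacker's AttackHitHandler.
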(fn ReceivedNotifyTick
  (params (MeshComp :type Skeletal%20Mesh%20Component%20Object%20Reference) (Animation :type Anim%20Sequence%20Base%20Object%20Reference) (FrameDeltaTime :type Float%20%28single-precision%29) (EventReference :type Anim%20Notify%20Event%20Reference%20Structure%20%28by%20ref%29))
  (bind _returnvalue (Components|GetOwner MeshComp))
  (bind _returnvalue_2 (Utilities|GetObjectName Animation))
  (bind _array (Utilities|Array|MakeArray "ObjectTypeQuery3"))
  (bind _returnvalue_3 (Components|GetOwner _returnvalue))
  (bind _array_2 (Utilities|Array|MakeArray _returnvalue_3))
  (bind _asaic_base_cat (Utilities|Casting|CastToAIC_BaseCat _returnvalue_3)
    (:then
      (bind _asbp_base_cat (Utilities|Casting|CastToBP_BaseCat (Pawn|GetControlledPawn _asaic_base_cat)))
      (if (Utilities|Enum|Equal(Enum) _returnvalue_2 "AM_Cat_Attack_3")
        (bind _outhits (Collision|MultiSphereTraceForObjects _asbp_base_cat (.location (Transformation|GetBoneTransform (Variables|/Script/Engine.Character|GetMesh _asbp_base_cat) "mouthSocket" "RTS_World")) (.location (Transformation|GetBoneTransform (Variables|/Script/Engine.Character|GetMesh _asbp_base_cat) "mouthSocket" "RTS_World")) 32.0 _array false _array_2 "ForOneFrame"))
        (for _array_element _outhits
          (if (== (Utilities|GetClass (.HitActor (Collision|BreakHitResult _array_element))) "/Game/Blueprints/Player/BP_Player.BP_Player_C")
            (Default|AttackHitHandler _asbp_base_cat (.HitActor (Collision|BreakHitResult _array_element)))
            (return true)))
        (elif (Utilities|Enum|Equal(Enum) _returnvalue_2 "AM_Cat_Attack_Left")
          (bind _outhits_2 (Collision|MultiSphereTraceForObjects _asbp_base_cat (.location (Transformation|GetBoneTransform (Variables|/Script/Engine.Character|GetMesh _asbp_base_cat) "claw_f_LSocket" "RTS_World")) (.location (Transformation|GetBoneTransform (Variables|/Script/Engine.Character|GetMesh _asbp_base_cat) "claw_f_LSocket" "RTS_World")) 32.0 _array false _array_2 "ForOneFrame"))
          (for _array_element_2 _outhits_2
            (if (== (Utilities|GetClass (.HitActor (Collision|BreakHitResult _array_element_2))) "/Game/Blueprints/Player/BP_Player.BP_Player_C")
              (Default|AttackHitHandler _asbp_base_cat (.HitActor (Collision|BreakHitResult _array_element_2)))
              (return true)))
          (else
            (bind _outhits_3 (Collision|MultiSphereTraceForObjects _asbp_base_cat (.location (Transformation|GetBoneTransform (Variables|/Script/Engine.Character|GetMesh _asbp_base_cat) "claw_f_RSocket" "RTS_World")) (.location (Transformation|GetBoneTransform (Variables|/Script/Engine.Character|GetMesh _asbp_base_cat) "claw_f_RSocket" "RTS_World")) 32.0 _array false _array_2 "ForOneFrame"))
            (for _array_element_3 _outhits_3
              (if (== (Utilities|GetClass (.HitActor (Collision|BreakHitResult _array_element_3))) "/Game/Blueprints/Player/BP_Player.BP_Player_C")
                (Default|AttackHitHandler _asbp_base_cat (.HitActor (Collision|BreakHitResult _array_element_3)))
                (return true)))))))
    (:CastFailed
      (bind _asplayer_controller (Utilities|Casting|CastToPlayerController _returnvalue_3))
      (bind _asbp_player (Utilities|Casting|CastToBP_Player (Pawn|GetControlledPawn _asplayer_controller)))
      (bind _outhits_4 (Collision|MultiSphereTraceForObjects _asbp_player (Transformation|GetSocketLocation (Variables|/Script/Engine.Character|GetMesh _asbp_player) "hand_rStartTrace") (Transformation|GetSocketLocation (Variables|/Script/Engine.Character|GetMesh _asbp_player) "hand_rEndTrace") 16.0 _array false (Actor|GetAttachedActors _asbp_player true false) "ForOneFrame"))
      (for _array_element_4 _outhits_4
        (if (and (!= (Utilities|GetClass (.HitActor (Collision|BreakHitResult _array_element_4))) "/Game/Blueprints/Player/BP_Player.BP_Player_C") (Utilities|DoesObjectImplementInterface (.HitActor (Collision|BreakHitResult _array_element_4)) "/Game/Blueprints/Interfaces/BPI_Damagable.BPI_Damagable_C"))
          (Default|AttackHitHandler _asbp_player (.HitActor (Collision|BreakHitResult _array_element_4)))
          (return true))))))