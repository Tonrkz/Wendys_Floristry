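; Player health component that holds HP and offers healing, passive regeneration and a debug readout.
; Heal adds to HP and clamps the result between zero and MaxHP.
; RegenerateHP adds RegenHP scaled by the passed-in delta, only while HP is below half of MaxHP.
; DisplayHealthData prints current and maximum HP as formatted text.
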(fn Heal
  (params (amount :type Float%20%28double-precision%29))
  (Variables|Default|SetHP (Math|Float|Clamp(Float) (+ (Variables|Default|GetHP) amount) 0.0 (Variables|Default|GetmaxHP)))
  (return))

(fn DisplayHealthData
  (Development|PrintText (Utilities|Text|FormatText "HP: {HP} | MaxHP: {maxHP}" (Variables|Default|GetHP) (Variables|Default|GetmaxHP)))
  (return))

(fn RegenerateHP
  (params (Delta :type Float%20%28double-precision%29))
  (if (< (Variables|Default|GetHP) (/ (Variables|Default|GetmaxHP) 2.0))
    (Variables|Default|SetHP (+ (Variables|Default|GetHP) (* Delta (Variables|Default|GetRegenHP))))
    (return)))