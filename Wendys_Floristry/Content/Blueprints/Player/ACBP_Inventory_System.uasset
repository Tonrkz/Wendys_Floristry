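; Player inventory component that stores flower counts by color in an array, checked against a slot limit and against customer orders.
; UseFlower spends the selected flower and notifies the overlay: red heals, blue grants temporary defense, yellow gives temporary speed, and orange has no effect.
; Selection is offset: the White case uses orange and the Orange case uses yellow.
; Effects reach the player through GetActorOfClass on BP_Player.
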(fn CheckInventory
  (Variables|Default|SetcountInventory 0)
  (for _array_element (Variables|Default|Getinventory)
    (Variables|Default|SetcountInventory (+ _array_element (Variables|Default|GetcountInventory))))
  (if (>= (Variables|Default|GetcountInventory) (Variables|Default|GetmaxInventory))
    (return true)
    (else
      (return false))))

(fn CheckInventoryforCustomer
  (params (RedWanted :type Byte) (BlueWanted :type Byte) (WhiteWanted :type Byte) (OrangeWanted :type Byte) (YellowWanted :type Byte) (PinkWanted :type Byte) (PurpleWanted :type Byte))
  (Utilities|Array|SetArrayElem (LocalVariables|GetWantedInventory) 0 RedWanted)
  (Utilities|Array|SetArrayElem (LocalVariables|GetWantedInventory) 1 BlueWanted)
  (Utilities|Array|SetArrayElem (LocalVariables|GetWantedInventory) 2 WhiteWanted)
  (Utilities|Array|SetArrayElem (LocalVariables|GetWantedInventory) 3 OrangeWanted)
  (Utilities|Array|SetArrayElem (LocalVariables|GetWantedInventory) 4 YellowWanted)
  (Utilities|Array|SetArrayElem (LocalVariables|GetWantedInventory) 5 PinkWanted)
  (Utilities|Array|SetArrayElem (LocalVariables|GetWantedInventory) 6 PurpleWanted)
  (bind (_array_element _array_index) (Utilities|Array|ForEachLoopwithBreak (Variables|Default|Getinventory) :!label _label)
    (:LoopBody
      (if (>= _array_element (Utilities|Array|Get(acopy) (LocalVariables|GetWantedInventory) _array_index))
        (LocalVariables|SetValidInventory true)
        (else
          (Development|PrintText (Utilities|Text|FormatText "Not Enough {Color} Flower!" (Utilities|String|EnumtoString (Utilities|Enum|LiteralenumEnum_Flower_Colors (Utilities|Enum|ByteToEnumEnum_Flower_Colors (Math|Conversions|ToByte(Integer) _array_index))))))
          (LocalVariables|SetValidInventory false)
          (goto _label Break))))
    (:Completed
      (return (LocalVariables|GetValidInventory)))))

(fn DisplayFlowerInventory
  (bind (_arrayindex _arrayelement) (Utilities|Array|ReverseforEachLoop (Variables|Default|Getinventory))
    (:LoopBody
      (Development|PrintText (Utilities|Text|FormatText "Flower: {Index} | Count: {Count}" (Utilities|String|EnumtoString (Utilities|Enum|ByteToEnumEnum_Ball_Colors (Math|Conversions|ToByte(Integer) _arrayindex))) _arrayelement)))
    (:Completed
      (return))))

(fn DisplayInventoryStat
  (bind _isinventoryfull (CallFunction|CheckInventory))
  (if _isinventoryfull
    (Development|PrintString "Inventory Full!"))
  (Development|PrintText (Utilities|Text|FormatText "Slots: {Count Inventory} | Max Slots: {Max Inventory}" (Variables|Default|GetcountInventory) (Variables|Default|GetmaxInventory))))

(fn AddFlowertoInventory
  (params (FlowerColor :type Enum_Flower_Colors%20Enum :default "NewEnumerator0"))
  (switch Utilities|FlowControl|Switch|SwitchonEnum_Flower_Colors FlowerColor
    (:NewEnumerator0
      (bind _output_get (Variables|Default|SetinventoryIndex 0))
      (Utilities|Array|SetArrayElem (Variables|Default|GetInventory) _output_get (+ (Utilities|Array|Get(acopy) (Variables|Default|GetInventory) _output_get) 1)))
    (:NewEnumerator1
      (bind _output_get_2 (Variables|Default|SetinventoryIndex 1))
      (Utilities|Array|SetArrayElem (Variables|Default|GetInventory) _output_get_2 (+ (Utilities|Array|Get(acopy) (Variables|Default|GetInventory) _output_get_2) 1)))
    (:NewEnumerator2
      (bind _output_get_3 (Variables|Default|SetinventoryIndex 2))
      (Utilities|Array|SetArrayElem (Variables|Default|GetInventory) _output_get_3 (+ (Utilities|Array|Get(acopy) (Variables|Default|GetInventory) _output_get_3) 1)))
    (:NewEnumerator3
      (bind _output_get_4 (Variables|Default|SetinventoryIndex 3))
      (Utilities|Array|SetArrayElem (Variables|Default|GetInventory) _output_get_4 (+ (Utilities|Array|Get(acopy) (Variables|Default|GetInventory) _output_get_4) 1)))
    (:NewEnumerator4
      (bind _output_get_5 (Variables|Default|SetinventoryIndex 4))
      (Utilities|Array|SetArrayElem (Variables|Default|GetInventory) _output_get_5 (+ (Utilities|Array|Get(acopy) (Variables|Default|GetInventory) _output_get_5) 1)))
    (:NewEnumerator5
      (bind _output_get_6 (Variables|Default|SetinventoryIndex 5))
      (Utilities|Array|SetArrayElem (Variables|Default|GetInventory) _output_get_6 (+ (Utilities|Array|Get(acopy) (Variables|Default|GetInventory) _output_get_6) 1)))
    (:NewEnumerator6
      (bind _output_get_7 (Variables|Default|SetinventoryIndex 6))
      (Utilities|Array|SetArrayElem (Variables|Default|GetInventory) _output_get_7 (+ (Utilities|Array|Get(acopy) (Variables|Default|GetInventory) _output_get_7) 1)))))

(fn UseFlower
  (params (OverlayGUI :type WBP%20Overlay%20GUI%20Object%20Reference))
  (switch Utilities|FlowControl|Switch|SwitchonEnum_Flower_Colors (Utilities|Enum|ByteToEnumEnum_Flower_Colors (Variables|Default|GetitemSelect))
    (:NewEnumerator0
      (CallFunction|UseRedFlower OverlayGUI))
    (:NewEnumerator1
      (CallFunction|UseBlueFlower OverlayGUI))
    (:NewEnumerator2
      (CallFunction|UseOrangeFlower OverlayGUI))
    (:NewEnumerator3
      (CallFunction|UseYellowFlower OverlayGUI)))
  (return))

(fn UseRedFlower
  (params (OverlayGUI :type WBP%20Overlay%20GUI%20Object%20Reference))
  (bind _result (Utilities|Text|FormatText "Red"))
  (bind _result_2 (Utilities|Text|FormatText "Not Enough {Color} Flower!" _result))
  (bind _result_3 (Utilities|Text|FormatText "Used {Color} Flower to Heal!" _result))
  (bind _output_get (Variables|Default|SetinventoryIndex 0))
  (if (>= (Utilities|Array|Get(acopy) (Variables|Default|GetInventory) _output_get) 1)
    (Utilities|Array|SetArrayElem (Variables|Default|GetInventory) _output_get (- (Utilities|Array|Get(acopy) (Variables|Default|GetInventory) _output_get) 1))
    (Development|PrintText _result_3)
    (Default|OnNoti OverlayGUI _result_3)
    (bind _returnvalue (Actor|GetActorOfClass "/Game/Blueprints/Player/BP_Player.BP_Player_C"))
    (Default|Heal (Variables|/Game/Blueprints/Player/BP_Player.BP_Player_C|GetACBP_Health_System _returnvalue) 1e+01)
    (return)
    (else
      (Development|PrintText _result_2)
      (Default|OnNoti OverlayGUI _result_2))))

(fn UseBlueFlower
  (params (OverlayGUI :type WBP%20Overlay%20GUI%20Object%20Reference))
  (bind _result (Utilities|Text|FormatText "Blue"))
  (bind _result_2 (Utilities|Text|FormatText "Not Enough {Color} Flower!" _result))
  (bind _result_3 (Utilities|Text|FormatText "Used {Color} Flower!" _result))
  (bind _output_get (Variables|Default|SetinventoryIndex 1))
  (if (>= (Utilities|Array|Get(acopy) (Variables|Default|GetInventory) _output_get) 1)
    (Utilities|Array|SetArrayElem (Variables|Default|GetInventory) _output_get (- (Utilities|Array|Get(acopy) (Variables|Default|GetInventory) _output_get) 1))
    (Development|PrintText _result_3)
    (Default|OnNoti OverlayGUI _result_3)
    (bind _returnvalue (Actor|GetActorOfClass "/Game/Blueprints/Player/BP_Player.BP_Player_C"))
    (Default|TempDef (Variables|/Game/Blueprints/Player/BP_Player.BP_Player_C|GetACBP_Status_System _returnvalue) 15 1e+01)
    (else
      (Development|PrintText _result_2)
      (Default|OnNoti OverlayGUI _result_2))))

(fn UseOrangeFlower
  (params (OverlayGUI :type WBP%20Overlay%20GUI%20Object%20Reference))
  (bind _result (Utilities|Text|FormatText "Orange"))
  (bind _result_2 (Utilities|Text|FormatText "Not Enough {Color} Flower!" _result))
  (bind _result_3 (Utilities|Text|FormatText "Used {Color} Flower!" _result))
  (bind _output_get (Variables|Default|SetinventoryIndex 3))
  (if (>= (Utilities|Array|Get(acopy) (Variables|Default|GetInventory) _output_get) 1)
    (Utilities|Array|SetArrayElem (Variables|Default|GetInventory) _output_get (- (Utilities|Array|Get(acopy) (Variables|Default|GetInventory) _output_get) 1))
    (Development|PrintText _result_3)
    (Default|OnNoti OverlayGUI _result_3)
    (bind _returnvalue (Actor|GetActorOfClass "/Game/Blueprints/Player/BP_Player.BP_Player_C"))
    (else
      (Development|PrintText _result_2)
      (Default|OnNoti OverlayGUI _result_2))))

(fn UseYellowFlower
  (params (OverlayGUI :type WBP%20Overlay%20GUI%20Object%20Reference))
  (bind _result (Utilities|Text|FormatText "Yellow"))
  (bind _result_2 (Utilities|Text|FormatText "Not Enough {Color} Flower!" _result))
  (bind _result_3 (Utilities|Text|FormatText "Used {Color} Flower!" _result))
  (bind _output_get (Variables|Default|SetinventoryIndex 4))
  (if (>= (Utilities|Array|Get(acopy) (Variables|Default|GetInventory) _output_get) 1)
    (Utilities|Array|SetArrayElem (Variables|Default|GetInventory) _output_get (- (Utilities|Array|Get(acopy) (Variables|Default|GetInventory) _output_get) 1))
    (Development|PrintText _result_3)
    (Default|OnNoti OverlayGUI _result_3)
    (bind _returnvalue (Actor|GetActorOfClass "/Game/Blueprints/Player/BP_Player.BP_Player_C"))
    (Default|TempSpeed _returnvalue 3e+01 1e+01)
    (return)
    (else
      (Development|PrintText _result_2)
      (Default|OnNoti OverlayGUI _result_2))))