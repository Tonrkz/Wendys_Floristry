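; Player status component that holds Defense, Attack and Harvest Speed stats and applies temporary buffs.
; TempDef and TempAtk add an amount to their stat, then subtract it after a timed Delay.
; Each event has a single Delay, so a call during an active buff adds again without scheduling another removal.
; DisplayPlayerStatus prints the three stats as formatted text; Harvest Speed is only displayed here.
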(event Custom|TempDef
  (params (Amount :type Integer) (Time :type Float%20%28double-precision%29))
  (Variables|Default|SetDEF (+ (Variables|Default|GetDEF) Amount))
  (Utilities|FlowControl|Delay Time)
  (Variables|Default|SetDEF (- (Variables|Default|GetDEF) Amount)))

(event Custom|TempAtk
  (params (Amount :type Integer) (Time :type Float%20%28double-precision%29))
  (bind _output_get (Variables|Default|SetATK (+ (Variables|Default|GetATK) Amount)))
  (Utilities|FlowControl|Delay Time)
  (Variables|Default|SetATK (- _output_get Amount)))

(fn DisplayPlayerStatus
  (Development|PrintText (Utilities|Text|FormatText "Defense: {DEF}" (Variables|Default|GetDEF)))
  (Development|PrintText (Utilities|Text|FormatText "Attack: {ATK}" (Variables|Default|GetATK)))
  (Development|PrintText (Utilities|Text|FormatText "Harvest Speed: {Harvest Speed}" (Variables|Default|GetharvestSpeed)))
  (return))