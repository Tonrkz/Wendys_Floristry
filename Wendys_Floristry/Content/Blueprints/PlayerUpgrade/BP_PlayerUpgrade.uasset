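; Interactable player upgrade station that opens the upgrade screen through BP_Player.
; On interact it waits InteractTime, then shows WBP_PlayerUpgradeScreen only if F is down at that moment, approximating a hold-to-interact.
; On BeginPlay it caches the day count from BP_DayNightCycle and fills UpgradeCost from UpgradeCount with a linear formula.
; The cached day count does not affect cost here.
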(event EventBeginPlay
  (CallFunction|GetDayCount)
  (CallFunction|CalculateUpgradeCost))

(event EventOnInteract
  (Utilities|FlowControl|Delay (Variables|Default|GetInteractTime))
  (if (Game|Player|IsInputKeyDown (Game|GetPlayerController 0) "F")
    (bind _returnvalue (Actor|GetActorOfClass "/Game/Blueprints/Player/BP_Player.BP_Player_C"))
    (Default|DisplayUI _returnvalue "/Game/Blueprints/Widgets/WBP_PlayerUpgradeScreen.WBP_PlayerUpgradeScreen_C")))

(fn ConstructionScript)

(fn GetDayCount
  (bind _returnvalue (Actor|GetActorOfClass "/Game/Blueprints/DayNightCycle/BP_DayNightCycle.BP_DayNightCycle_C"))
  (Variables|Default|SetDayCount (Variables|/Game/Blueprints/DayNightCycle/BP_DayNightCycle.BP_DayNightCycle_C|GetdayCount _returnvalue))
  (return))

(fn CalculateUpgradeCost
  (for (_ _array_index) (Variables|Default|GetUpgradeCost)
    (bind _cost (CallFunction|GetCost (Utilities|Array|Get(acopy) (Variables|Default|GetUpgradeCount) _array_index)))
    (Utilities|Array|SetArrayElem (Variables|Default|GetUpgradeCost) _array_index _cost))
  (return))

(fn GetCost
  (params (Count :type Integer))
  (bind _output_get (LocalVariables|SetNumber_1 (+ 1 (* Count 2))))
  (return _output_get))