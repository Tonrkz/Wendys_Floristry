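; Map controller that randomizes and regenerates the PCG actors in its PCGFlower array and toggles their in-game visibility.
; ShowPCGV unhides each actor, cleans up its PCG component, assigns a random seed and generates locally, printing the seed for debugging.
; On BeginPlay it runs ShowPCGV, then hides the actors one second later.
; Separate events regenerate without hiding (GeneratePCG) or clean up the generated content (ClearPCGV).
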(event Custom|TriggerPCGV
  (CallFunction|ShowPCGV)
  (Utilities|FlowControl|Delay 1.0)
  (CallFunction|HidePCGV))

(event Custom|ClearPCGV
  (for _array_element (Variables|Default|GetPCGFlower)
    (Class|PCGComponent|CleanupLocal (Variables|/Script/PCG.PCGVolume|GetPCGComponent _array_element) false false)))

(event Custom|GeneratePCG
  (CallFunction|ShowPCGV))

(event EventBeginPlay
  (CallFunction|TriggerPCGV))

(fn ConstructionScript)

(fn HidePCGV
  (for _array_element (Variables|Default|GetPCGFlower)
    (Rendering|SetActorHiddenInGame _array_element true)
    (Development|PrintText (Utilities|Text|FormatText "{Name}: Hidden" (Utilities|GetDisplayName _array_element))))
  (return))

(fn ShowPCGV
  (for _array_element (Variables|Default|GetPCGFlower)
    (bind _output_get (Variables|Default|SetSeed (Math|Random|RandomIntegerinRange -90000000 90000000)))
    (Rendering|SetActorHiddenInGame _array_element false)
    (Class|PCGComponent|CleanupLocal (Variables|/Script/PCG.PCGVolume|GetPCGComponent _array_element) false false)
    (bind _output_get_2 (Variables|/Script/PCG.PCGComponent|SetSeed (Variables|/Script/PCG.PCGVolume|GetPCGComponent _array_element) _output_get))
    (Class|PCGComponent|GenerateLocal (Variables|/Script/PCG.PCGVolume|GetPCGComponent _array_element) true)
    (Development|PrintText (Utilities|Text|FormatText "{Name}: Shown | Seed: {Seed}" (Utilities|GetDisplayName _array_element) _output_get_2)))
  (return))